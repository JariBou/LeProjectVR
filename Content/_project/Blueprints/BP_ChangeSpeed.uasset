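; Box trigger volume, likely a water current, that changes the BP_Radal boat's min and max speed while inside.
; Overlap increments the boat's water-flow counter; exit restores the normal speeds cached at BeginPlay only when that counter is at most one.
; Tick blends limits over separate in/out times and clamps velocity, borrowing a hand/tracker enum as transition state (Left in, Right out, Gun idle).
; An older timeline lerp remains unconnected.
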(event Collision|EventActorEndOverlap
  (params (OtherActor :type Actor%20Object%20Reference))
  (bind _asbp_radal (Utilities|Casting|CastToBP_Radal OtherActor))
  (bind _output_get (Variables|Default|SetAs%20BP%20Radal _asbp_radal))
  (if (<= (Variables|/Game/_project/Blueprints/BP_Radal.BP_Radal_C|GetNbTriggerWaterFlow _output_get) 1)
    (Variables|Default|SetLastMinSpeed (Variables|Default|GetNormalMinSpeed))
    (Variables|Default|SetLastMaxSpeed (Variables|Default|GetNormalMaxSpeed))
    (Variables|Default|SetAccelType "Right")
    (Variables|Default|SetTimer 0.0)))

(event Collision|EventActorBeginOverlap
  (params (OtherActor :type Actor%20Object%20Reference))
  (bind _asbp_radal (Utilities|Casting|CastToBP_Radal OtherActor))
  (bind _output_get (Variables|Default|SetAs%20BP%20Radal _asbp_radal))
  (Math|Integer|IncrementInt (Variables|/Game/_project/Blueprints/BP_Radal.BP_Radal_C|GetNbTriggerWaterFlow _output_get)
    (:%20%20
      (Variables|Default|SetLastMinSpeed (Variables|/Game/_project/Blueprints/BP_Radal.BP_Radal_C|GetMinSpeed _output_get))
      (Variables|Default|SetLastMaxSpeed (Variables|/Game/_project/Blueprints/BP_Radal.BP_Radal_C|GetMaxSpeed _output_get))
      (Variables|Default|SetAccelType "Left")
      (Variables|Default|SetTimer 0.0))))

(event EventTick
  (params (DeltaSeconds :type Float%20%28single-precision%29))
  (if (Utilities|Enum|NotEqual(Enum) (Variables|Default|GetAccelType) "Gun")
    (bind _output_get (Variables|Default|SetTimer (+ DeltaSeconds (Variables|Default|GetTimer))))
    (if (<= _output_get (Utilities|Select :Index (Variables|Default|GetAccelType) :Left (Variables|Default|GetInTransitionTime) :Right (Variables|Default|GetOutTransitionTime) :AnyHand 0.0 :Pad 0.0 :ExternalCamera 0.0 :Gun 0.0 :HMD 0.0 :Chest 0.0 :LeftShoulder 0.0 :RightShoulder 0.0 :LeftElbow 0.0 :RightElbow 0.0 :Waist 0.0 :LeftKnee 0.0 :RightKnee 0.0 :LeftFoot 0.0 :RightFoot 0.0 :Special 0.0))
      (CallFunction|ChangeBoatSpeed (Math|Float|SelectFloat (/ _output_get (Utilities|Select :Index (Variables|Default|GetAccelType) :Left (Variables|Default|GetInTransitionTime) :Right (Variables|Default|GetOutTransitionTime) :AnyHand 0.0 :Pad 0.0 :ExternalCamera 0.0 :Gun 0.0 :HMD 0.0 :Chest 0.0 :LeftShoulder 0.0 :RightShoulder 0.0 :LeftElbow 0.0 :RightElbow 0.0 :Waist 0.0 :LeftKnee 0.0 :RightKnee 0.0 :LeftFoot 0.0 :RightFoot 0.0 :Special 0.0)) (- 1.0 (/ _output_get (Utilities|Select :Index (Variables|Default|GetAccelType) :Left (Variables|Default|GetInTransitionTime) :Right (Variables|Default|GetOutTransitionTime) :AnyHand 0.0 :Pad 0.0 :ExternalCamera 0.0 :Gun 0.0 :HMD 0.0 :Chest 0.0 :LeftShoulder 0.0 :RightShoulder 0.0 :LeftElbow 0.0 :RightElbow 0.0 :Waist 0.0 :LeftKnee 0.0 :RightKnee 0.0 :LeftFoot 0.0 :RightFoot 0.0 :Special 0.0))) (Utilities|Enum|Equal(Enum) (Variables|Default|GetAccelType) "Left")))
      (else
        (CallFunction|ChangeBoatSpeed (Utilities|Select :Index (Variables|Default|GetAccelType) :Left 1.0 :Right 0.0 :AnyHand 0.0 :Pad 0.0 :ExternalCamera 0.0 :Gun 0.0 :HMD 0.0 :Chest 0.0 :LeftShoulder 0.0 :RightShoulder 0.0 :LeftElbow 0.0 :RightElbow 0.0 :Waist 0.0 :LeftKnee 0.0 :RightKnee 0.0 :LeftFoot 0.0 :RightFoot 0.0 :Special 0.0))
        (Variables|Default|SetAccelType "Gun")))))

(event EventBeginPlay
  (bind _returnvalue (Actor|GetActorOfClass "/Game/_project/Blueprints/BP_Radal.BP_Radal_C"))
  (Variables|Default|SetNormalMinSpeed (Variables|/Game/_project/Blueprints/BP_Radal.BP_Radal_C|GetMinSpeed _returnvalue))
  (Variables|Default|SetNormalMaxSpeed (Variables|/Game/_project/Blueprints/BP_Radal.BP_Radal_C|GetMaxSpeed _returnvalue))
  (Variables|Default|SetAccelType "Gun"))

(fn ConstructionScript
  (Components|Box|SetBoxExtent (Variables|Default|GetBox) (Variables|Default|GetBoxExtent) true))

(fn ChangeBoatSpeed
  (params (Alpha :type Float%20%28double-precision%29))
  (bind _as_bp_radal (Variables|Default|GetAs%20BP%20Radal))
  (bind _output_get (Variables|/Game/_project/Blueprints/BP_Radal.BP_Radal_C|SetMinSpeed _as_bp_radal (Math|Float|Lerp (Variables|Default|GetLastMinSpeed) (Variables|Default|GetNewMinSpeed) Alpha)))
  (bind _output_get_2 (Variables|/Game/_project/Blueprints/BP_Radal.BP_Radal_C|SetMaxSpeed _as_bp_radal (Math|Float|Lerp (Variables|Default|GetLastMaxSpeed) (Variables|Default|GetNewMaxSpeed) Alpha)))
  (Variables|/Game/_project/Blueprints/BP_Radal.BP_Radal_C|SetVelocity _as_bp_radal (Math|Vector|ClampVectorSize (Variables|/Game/_project/Blueprints/BP_Radal.BP_Radal_C|GetVelocity (Variables|Default|GetAs%20BP%20Radal)) _output_get _output_get_2)))