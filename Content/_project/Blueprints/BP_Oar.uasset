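; VR oar actor with two grab components for one- or two-handed holding.
; The first grab disables physics and attaches the oar to that motion controller, while a grab on the other component registers the second hand.
; With both held, Tick aligns the oar along the line between controllers, mixing in the first controller's roll.
; Releasing the first grip detaches it, restores physics and clears both grips.
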(event OnGrabbed(BP_GrabComponent)
  (params (MotionController :type Motion%20Controller%20Component%20Object%20Reference) (ActorGrabbed :type Actor%20Object%20Reference))
  ;[0.15 0.15 0.15 0.5] Grab / release inputs
  (CallFunction|GrabOar MotionController (Variables|Default|GetBP_GrabComponent)))

(event OnGrabbed(BP_GrabComponent1)
  (params (MotionController :type Motion%20Controller%20Component%20Object%20Reference) (ActorGrabbed :type Actor%20Object%20Reference))
  ;[0.15 0.15 0.15 0.5] Grab / release inputs
  (CallFunction|GrabOar MotionController (Variables|Default|GetBP_GrabComponent1)))

(event OnDropped(BP_GrabComponent)
  (params (ActorDropped :type Actor%20Object%20Reference))
  ;[0.15 0.15 0.15 0.5] Grab / release inputs
  (CallFunction|ReleaseOar 0 (Variables|Default|GetBP_GrabComponent)))

(event OnDropped(BP_GrabComponent1)
  (params (ActorDropped :type Actor%20Object%20Reference))
  ;[0.15 0.15 0.15 0.5] Grab / release inputs
  (CallFunction|ReleaseOar 0 (Variables|Default|GetBP_GrabComponent1)))

(event EventTick
  (params (DeltaSeconds :type Float%20%28single-precision%29))
  (bind _firstgripcontroller (Variables|Default|GetFirstGripController))
  (bind _secondgripcontroller (Variables|Default|GetSecondGripController))
  (bind _returnvalue (Transformation|GetWorldLocation _secondgripcontroller))
  (bind _returnvalue_2 (Transformation|GetWorldLocation _firstgripcontroller))
  (bind _returnvalue_3 (Math|Rotator|FindLookatRotation _returnvalue_2 _returnvalue))
  (bind _returnvalue_4 (Math|Rotator|CombineRotators _returnvalue_3 "0.000000,-90.000000,0.000000"))
  ;[0.15 0.15 0.15 0.5] Angle if both hands grabbed
  (if (and (Utilities|IsValid (Variables|Default|GetFirstGrabComponentRef)) (Utilities|IsValid (Variables|Default|GetSecondGrabComponentRef)))
    (Transformation|SetActorRotation (Math|Rotator|MakeRotator (* (.pitch _returnvalue_4) -1.0) (.roll (Transformation|GetWorldRotation _firstgripcontroller)) (.yaw _returnvalue_4)))))

(fn ConstructionScript)

(fn GrabOar
  (params (MotionController :type Motion%20Controller%20Component%20Object%20Reference) (GrabComponent :type BP%20Grab%20Component%20Object%20Reference))
  (Variables|Default|GetFirstGrabComponentRef
    (:then
      ;[0.15 0.15 0.15 0.5] Setup second reference
      (if (not (== GrabComponent (Variables|Default|GetFirstGrabComponentRef)))
        (Variables|Default|SetSecondGrabComponentRef GrabComponent)
        (Variables|Default|SetSecondGripController MotionController)))
    (:else
      ;[0.15 0.15 0.15 0.5] Attach the oar to the first hand
      (Variables|Default|SetFirstGrabComponentRef GrabComponent)
      (bind _output_get (Variables|Default|SetFirstGripController MotionController))
      (Physics|SetSimulatePhysics (Variables|Default|GetCylinder) false)
      (bind _returnvalue (Transformation|AttachComponentToComponent _output_get "None" "KeepWorld" "KeepWorld" "KeepWorld" true))
      (if (not _returnvalue)
        (Development|PrintString "Oar attachement failed")))))

(fn ReleaseOar
  (params (MotionControllerRef :type Motion%20Controller%20Component%20Object%20Reference) (GrabComponent :type BP%20Grab%20Component%20Object%20Reference))
  ;[0.15 0.15 0.15 0.5] Detach from hand if is the first
  (if (== GrabComponent (Variables|Default|GetFirstGrabComponentRef))
    (Transformation|DetachFromActor "KeepWorld" "KeepWorld" "KeepWorld")
    (Physics|SetSimulatePhysics (Variables|Default|GetCylinder) true)
    (Variables|Default|SetFirstGripController 0)
    (Variables|Default|SetFirstGrabComponentRef 0))
  ;[0.15 0.15 0.15 0.5] Else dereference second
  (Variables|Default|SetSecondGrabComponentRef 0)
  (Variables|Default|SetSecondGripController 0))