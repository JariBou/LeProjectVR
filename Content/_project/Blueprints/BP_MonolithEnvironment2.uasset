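; BP_MonolithEnvironment2 is a monolith environment piece whose emissive glow fades between off and on power levels.
; BeginPlay creates a dynamic material on the static mesh's first slot and sets the off intensity.
; CallFX plays a timeline whose curve lerps the "Emsissive_Intensity" parameter toward the on level, and EndFX reverses it.
; Each timeline update also prints the playback direction.
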(event EventCallFX
  (bind (_direction _courbe) (Timeline|AGOUGOUGAGA Play)
    (:Update
      (Development|PrintString (Utilities|String|EnumtoString _direction)))
    (:Finished
      _))
  (Rendering|Material|SetScalarParameterValue (Variables|Default|GetDynamic) "Emsissive_Intensity" (Math|Float|Lerp (Variables|Default|GetOffEmissivePower) (Variables|Default|GetOnEmissivePower) _courbe) :!class /Script/Engine.MaterialInstanceDynamic))

(event EventEndFX
  (bind (_direction _courbe) (Timeline|AGOUGOUGAGA Reverse)
    (:Update
      (Development|PrintString (Utilities|String|EnumtoString _direction)))
    (:Finished
      _))
  (Rendering|Material|SetScalarParameterValue (Variables|Default|GetDynamic) "Emsissive_Intensity" (Math|Float|Lerp (Variables|Default|GetOffEmissivePower) (Variables|Default|GetOnEmissivePower) _courbe) :!class /Script/Engine.MaterialInstanceDynamic))

(event EventBeginPlay
  (bind _staticmesh (Variables|Default|GetStaticMesh))
  (bind _returnvalue (Rendering|Material|CreateDynamicMaterialInstance _staticmesh 0 (Rendering|Material|GetMaterial _staticmesh 0) "None" :!class /Script/Engine.PrimitiveComponent))
  (bind _output_get (Variables|Default|SetDynamic _returnvalue))
  (Rendering|Material|SetScalarParameterValue _output_get "Emsissive_Intensity" (Variables|Default|GetOffEmissivePower) :!class /Script/Engine.MaterialInstanceDynamic))

(fn ConstructionScript)