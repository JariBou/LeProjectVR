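; BP_SpawnerTrigger is a trigger that spawns random trash items the first time a BP_Radal enters its detection volume.
; It picks a random count from ItemCountRange and, for each item, tells a randomly chosen entry in Spawners to spawn a random trash item.
; A HasSpawned flag makes it fire only once, and the same spawner can be picked repeatedly.
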(event OnComponentBeginOverlap(PlayerDetection)
  (params (OverlappedComponent :type Primitive%20Component%20Object%20Reference) (OtherActor :type Actor%20Object%20Reference) (OtherComp :type Primitive%20Component%20Object%20Reference) (OtherBodyIndex :type Integer) (bFromSweep :type Boolean) (SweepResult :type Hit%20Result%20Structure%20%28by%20ref%29))
  (if (not (Variables|Default|GetHasSpawned))
    (Utilities|Casting|CastToBP_Radal OtherActor)
    (CallFunction|SpawnItems)
    (Variables|Default|SetHasSpawned true)))

(event Custom|SpawnItems
  (bind _itemcountrange (Variables|Default|GetItemCountRange))
  (for _index (range 1 (Math|Random|RandomIntegerinRange (Math|Float|Floor (.x _itemcountrange)) (Math|Float|Ceil (.y _itemcountrange))))
    (Default|CESpawnRandomTrashItem (.OutItem (Utilities|Array|Random (Variables|Default|GetSpawners))))))

(fn ConstructionScript)