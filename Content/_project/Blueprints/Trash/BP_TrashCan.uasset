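; BP_TrashCan is a trash bin that collects trash dropped from an overlapping BP_Oar and shows its fill level.
; On box overlap it takes the oar's trash, pulls it into the cube with a timeline, destroys it, then re-allows drops after a one-second cooldown.
; Adding or removing levels restarts the Niagara effect and timeline-animates the cube's clamped Z scale from the trash count, with a deposit sound on adds.
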(event OnComponentBeginOverlap(Box)
  (params (OverlappedComponent :type Primitive%20Component%20Object%20Reference) (OtherActor :type Actor%20Object%20Reference) (OtherComp :type Primitive%20Component%20Object%20Reference) (OtherBodyIndex :type Integer) (bFromSweep :type Boolean) (SweepResult :type Hit%20Result%20Structure%20%28by%20ref%29))
  (if (Variables|Default|GetCanDrop)
    (bind _asbp_oar (Utilities|Casting|CastToBP_Oar OtherActor))
    (bind (_trash _foundthrash) (Default|DropIntoBasket _asbp_oar))
    (if _foundthrash
      (Variables|Default|SetCanDrop false)
      (Utilities|Time|SetTimerbyEvent (delegate Custom|CE_ReactivateDrop) 1.0)
      (CallFunction|AddTrashLevel 1)
      (bind _newtrack_0 (Timeline|BigJuicyMovement PlayFromStart)
        (:Update
          (Transformation|SetActorLocation _trash (Math|Vector|Lerp(Vector) (Transformation|GetActorLocation _trash) (Transformation|GetWorldLocation (Variables|Default|GetCube)) _newtrack_0) false false))
        (:Finished
          (Actor|DestroyActor _trash)
          (Components|Activation|Deactivate (Variables|Default|GetNS_Trash)))))))

(event Custom|CE_ReactivateDrop
  (Variables|Default|SetCanDrop true))

(event Custom|Baptiste_removeTrashLevel
  (params (NumberOfTimes :type Integer))
  (bind _ns_trash (Variables|Default|GetNS_Trash))
  (bind _cube (Variables|Default|GetCube))
  (bind _returnvalue (Transformation|GetWorldScale _cube))
  (Niagara|ResetSystem _ns_trash)
  (Components|Activation|Activate _ns_trash false)
  (for _index (range 0 (- NumberOfTimes 1))
    (Math|Integer|DecrementInt (Variables|Default|GetTrashLevel)))
  (Variables|Default|SetScaleZSave (.z _returnvalue))
  (bind _newtrack_0 (Timeline|BigJuicyBommchakalaka2 PlayFromStart)
    (:Update
      (Transformation|SetWorldScale3D _cube (Math|Vector|MakeVector (.x _returnvalue) (.y _returnvalue) (Math|Float|Clamp(Float) (Math|Float|Lerp (Variables|Default|GetScaleZSave) (* (Variables|Default|GetScaleAugmentPerTrash) (Variables|Default|GetTrashLevel)) _newtrack_0)))))))

(event Custom|AddTrashLevel
  (params (NumberOfTimes :type Integer))
  (bind _ns_trash (Variables|Default|GetNS_Trash))
  (bind _cube (Variables|Default|GetCube))
  (bind _returnvalue (Transformation|GetWorldScale _cube))
  (Niagara|ResetSystem _ns_trash)
  (Components|Activation|Activate _ns_trash false)
  ;[0.15 0.15 0.15 0.5] Sound
  (bind _soundtrashdepot (Variables|Default|GetSoundTrashDepot)
    (:then
      (Audio|SpawnSoundatLocation _soundtrashdepot (Transformation|GetActorLocation) "0, 0, 0" 1.0 1.0 0.0 0 0))
    (:else
      (Development|PrintString "Sound depot not present")))
  (for _index (range 0 (- NumberOfTimes 1))
    (Math|Integer|IncrementInt (Variables|Default|GetTrashLevel)))
  (Variables|Default|SetScaleZSave (.z _returnvalue))
  (bind _newtrack_0 (Timeline|BigJuicyBommchakalaka PlayFromStart)
    (:Update
      (Transformation|SetWorldScale3D _cube (Math|Vector|MakeVector (.x _returnvalue) (.y _returnvalue) (Math|Float|Clamp(Float) (Math|Float|Lerp (Variables|Default|GetScaleZSave) (+ 0.0 (* (Variables|Default|GetScaleAugmentPerTrash) (Variables|Default|GetTrashLevel))) _newtrack_0)))))))

(event EventBeginPlay
  (Components|Activation|Deactivate (Variables|Default|GetNS_Trash)))

(fn ConstructionScript)