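; BP_Trash is a physics-simulated trash actor that the player can catch with an oar.
; The construction script assigns its mesh from a variable and enables physics simulation.
; On overlap with a BP_Oar, it asks the oar to catch it; if that succeeds, it marks itself caught and disables physics and collision so it is not caught again.
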(event OnComponentBeginOverlap(StaticMesh)
  (params (OverlappedComponent :type Primitive%20Component%20Object%20Reference) (OtherActor :type Actor%20Object%20Reference) (OtherComp :type Primitive%20Component%20Object%20Reference) (OtherBodyIndex :type Integer) (bFromSweep :type Boolean) (SweepResult :type Hit%20Result%20Structure%20%28by%20ref%29))
  (if (not (Variables|Default|GetIsCaught))
    (bind _asbp_oar (Utilities|Casting|CastToBP_Oar OtherActor))
    (bind _caught (Default|CatchObject _asbp_oar self))
    (if _caught
      (Variables|Default|SetIsCaught true)
      (Physics|SetSimulatePhysics (Variables|Default|GetStaticMesh) false)
      (Collision|SetCollisionEnabled (Variables|Default|GetStaticMesh) "NoCollision"))))

(event EventBeginPlay)

(event Collision|EventActorBeginOverlap
  (params (OtherActor :type Actor%20Object%20Reference)))

(event EventTick
  (params (DeltaSeconds :type Float%20%28single-precision%29)))

(fn ConstructionScript
  (Components|StaticMesh|SetStaticMesh (Variables|Default|GetStaticMesh) (Variables|Default|GetMesh))
  (Physics|SetSimulatePhysics (Variables|Default|GetStaticMesh) true))