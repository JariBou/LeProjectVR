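; BP_Spawner is a placed spawn point that queues trash item requests and spawns them around itself.
; Each CE_SpawnRandomTrashItem call increments a pending count, spawning immediately if no cooldown is running, while Tick counts the cooldown down and drains the queue one item per second.
; Spawns are delegated to the level's BP_MasterSpawner at a random XY offset within RandomSpawnRange, a square area that the construction script previews as a sphere radius.
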(event Custom|CE_SpawnRandomTrashItem
  (Math|Integer|IncrementInt (Variables|Default|GetNbItemsToSpawn)
    (:%20%20
      (if (not (> (Variables|Default|GetSpawnCooldown) 0.0))
        (CallFunction|SpawnRandomTrashatSelf)))))

(event Custom|CheckAndSpawnIfNeeded
  (if (> (Variables|Default|GetNbItemsToSpawn) 0)
    (CallFunction|SpawnRandomTrashatSelf)))

(event EventBeginPlay
  (bind _returnvalue (Actor|GetActorOfClass "/Game/_project/Blueprints/Trash/BP_MasterSpawner.BP_MasterSpawner_C"))
  (Variables|Default|SetMasterSpawner _returnvalue))

(event EventTick
  (params (DeltaSeconds :type Float%20%28single-precision%29))
  (if (> (Variables|Default|GetSpawnCooldown) 0.0)
    (Variables|Default|SetSpawnCooldown (- (Variables|Default|GetSpawnCooldown) DeltaSeconds))
    (else
      (CallFunction|CheckandSpawnifNeeded))))

(fn ConstructionScript
  (Components|Sphere|SetSphereRadius (Variables|Default|GetSphere) (Variables|Default|GetRandomSpawnRange) true))

(fn SpawnRandomTrashatSelf
  (bind _returnvalue (Transformation|GetActorTransform))
  (bind _randomspawnrange (Variables|Default|GetRandomSpawnRange))
  (bind _returnvalue_2 (* _randomspawnrange -1.0))
  (Default|SpawnRandomItem (Variables|Default|GetMasterSpawner) (Math|Transform|MakeTransform (+ (Math|Vector|MakeVector (Math|Random|RandomFloatinRange _returnvalue_2 _randomspawnrange) (Math|Random|RandomFloatinRange _returnvalue_2 _randomspawnrange) 0.0) (.location _returnvalue)) (.rotation _returnvalue) (.scale _returnvalue)))
  (Variables|Default|SetSpawnCooldown 1.0)
  (Math|Integer|DecrementInt (Variables|Default|GetNbItemsToSpawn)))