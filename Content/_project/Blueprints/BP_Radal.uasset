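; VR paddled raft that carries the player pawn and a trash can.
; Side overlaps with the oar start a timer sampling its relative stroke, with delayed release to absorb physics flicker.
; Tick turns strokes into a Velocity variable with side-dependent lateral push, braking and drag, without moving the actor itself.
; Front obstacle hits zero forward speed and, when fast enough, remove a share of the trash.
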(event OnComponentBeginOverlap(Right)
  (params (OverlappedComponent :type Primitive%20Component%20Object%20Reference) (OtherActor :type Actor%20Object%20Reference) (OtherComp :type Primitive%20Component%20Object%20Reference) (OtherBodyIndex :type Integer) (bFromSweep :type Boolean) (SweepResult :type Hit%20Result%20Structure%20%28by%20ref%29))
  (bind _asbp_oar (Utilities|Casting|CastToBP_Oar OtherActor))
  (Variables|Default|SetAs%20BP%20Oar _asbp_oar)
  (Utilities|FlowControl|Sequence
    (:then_0
      (Utilities|Time|ClearandInvalidateTimerbyHandle (Variables|Default|GetUnlockPaddleHandle)))
    (:then_1
      (Variables|Default|SetOarPaddle OtherComp)
      (if (not (Utilities|Time|IsValidTimerHandle (Variables|Default|GetUpdateRotationHandle)))
        (Default|CallOnStartPagaieing)
        (bind _returnvalue (Utilities|Time|SetTimerbyFunctionName 0 "UpdateLocation" (Variables|Default|GetTimeToPad) true true))
        (Variables|Default|SetUpdateRotationHandle _returnvalue)
        (Variables|Default|SetPreviousOarPos (.ReturnValue_Location (Utilities|GetBpOarPadRelativeLoc)))
        (Variables|Default|SetSidePaddled "Right")))))

(event OnComponentEndOverlap(Right)
  (params (OverlappedComponent :type Primitive%20Component%20Object%20Reference) (OtherActor :type Actor%20Object%20Reference) (OtherComp :type Primitive%20Component%20Object%20Reference) (OtherBodyIndex :type Integer))
  (Utilities|Casting|CastToBP_Oar OtherActor)
  (Utilities|FlowControl|Sequence
    (:then_0
      (bind _returnvalue (Utilities|Time|SetTimerbyFunctionName 0 "UnlockPaddle" (Variables|Default|GetTimeToRelease)))
      (Variables|Default|SetUnlockPaddleHandle _returnvalue))))

(event OnComponentBeginOverlap(Left)
  (params (OverlappedComponent :type Primitive%20Component%20Object%20Reference) (OtherActor :type Actor%20Object%20Reference) (OtherComp :type Primitive%20Component%20Object%20Reference) (OtherBodyIndex :type Integer) (bFromSweep :type Boolean) (SweepResult :type Hit%20Result%20Structure%20%28by%20ref%29))
  (bind _asbp_oar (Utilities|Casting|CastToBP_Oar OtherActor))
  (Variables|Default|SetAs%20BP%20Oar _asbp_oar)
  (Utilities|FlowControl|Sequence
    (:then_0
      (Utilities|Time|ClearandInvalidateTimerbyHandle (Variables|Default|GetUnlockPaddleHandle)))
    (:then_1
      (Variables|Default|SetOarPaddle OtherComp)
      (if (not (Utilities|Time|IsValidTimerHandle (Variables|Default|GetUpdateRotationHandle)))
        (bind _returnvalue (Utilities|Time|SetTimerbyFunctionName 0 "UpdateLocation" (Variables|Default|GetTimeToPad) true true))
        (Variables|Default|SetUpdateRotationHandle _returnvalue)
        (Variables|Default|SetPreviousOarPos (.ReturnValue_Location (Utilities|GetBpOarPadRelativeLoc)))
        (Variables|Default|SetSidePaddled "Left")))))

(event OnComponentEndOverlap(Left)
  (params (OverlappedComponent :type Primitive%20Component%20Object%20Reference) (OtherActor :type Actor%20Object%20Reference) (OtherComp :type Primitive%20Component%20Object%20Reference) (OtherBodyIndex :type Integer))
  (Utilities|Casting|CastToBP_Oar OtherActor)
  (Utilities|FlowControl|Sequence
    (:then_0
      (bind _returnvalue (Utilities|Time|SetTimerbyFunctionName 0 "UnlockPaddle" (Variables|Default|GetTimeToRelease)))
      (Variables|Default|SetUnlockPaddleHandle _returnvalue))))

(event OnComponentBeginOverlap(FrontCollisionDetection)
  (params (OverlappedComponent :type Primitive%20Component%20Object%20Reference) (OtherActor :type Actor%20Object%20Reference) (OtherComp :type Primitive%20Component%20Object%20Reference) (OtherBodyIndex :type Integer) (bFromSweep :type Boolean) (SweepResult :type Hit%20Result%20Structure%20%28by%20ref%29))
  (bind _trashcanobj (Variables|Default|GetTrashCanObj))
  (if (Actor|ActorHasTag OtherActor "Obstacle")
    (Variables|Default|SetHasHitObstacle true)
    (if (>= (.y (Variables|Default|GetVelocity)) (Variables|BoomShakalaka|GetMinSpeedForCollisionDamage))
      (Default|CallOnCollision)
      (Default|BaptisteRemoveTrashLevel _trashcanobj (Math|Float|Floor (* (Variables|/Game/_project/Blueprints/Trash/BP_TrashCan.BP_TrashCan_C|GetTrashLevel _trashcanobj) (Variables|BoomShakalaka|GetPercentOfTrashLostOnCollision)))))))

(event OnComponentEndOverlap(FrontCollisionDetection)
  (params (OverlappedComponent :type Primitive%20Component%20Object%20Reference) (OtherActor :type Actor%20Object%20Reference) (OtherComp :type Primitive%20Component%20Object%20Reference) (OtherBodyIndex :type Integer))
  (if (Actor|ActorHasTag OtherActor "Obstacle")
    (Variables|Default|SetHasHitObstacle false)))

(event EventBeginPlay
  (bind _trashcan (Variables|Default|GetTrashCan))
  (bind _childactor (Variables|/Script/Engine.ChildActorComponent|GetChildActor _trashcan))
  (bind _returnvalue (Actor|GetActorOfClass "/Game/_project/Blueprints/BP_VRPawn.BP_VRPawn_C"))
  (Transformation|AttachActorToActor _returnvalue self "None" "KeepWorld" "KeepWorld" "KeepWorld" true)
  (Utilities|FlowControl|DelayUntilNextTick)
  (Utilities|IsValid _childactor
    (:Is%20Valid
      (bind _asbp_trash_can (Utilities|Casting|CastToBP_TrashCan _childactor))
      (bind _output_get (Variables|Default|SetTrashCanObj _asbp_trash_can))
      (Default|AddTrashLevel _output_get 10))))

(event EventTick
  (params (DeltaSeconds :type Float%20%28single-precision%29))
  (bind _paddlebreakingforcemultiplier (Variables|Movement|GetPaddleBreakingForceMultiplier))
  (bind _dragforce (Variables|Movement|GetDragForce))
  (bind _forwardacceleration (Variables|Default|GetForwardAcceleration))
  (bind _returnvalue (>= _forwardacceleration 0.0))
  (bind _returnvalue_2 (Math|Float|SelectFloat 1.0 _paddlebreakingforcemultiplier _returnvalue))
  (bind _returnvalue_3 (* _dragforce _returnvalue_2))
  (bind _returnvalue_4 (* DeltaSeconds _returnvalue_3))
  (if (Variables|Default|GetIsPadInWater)
    (if (> (Math|Float|Absolute(Float) (Variables|Default|GetForwardAcceleration)) 0.0)
      (if (> (Variables|Default|GetForwardAcceleration) 0.0)
        (CallFunction|UpdateForwardPaddling)
        (else
          (CallFunction|UpdateBackwardPaddling DeltaSeconds)))
      (else
        (Variables|Default|SetVelocity (Math|Vector|MakeVector (.x (+ (Math|Vector|NegateVector (Math|Vector|MakeVector (* _returnvalue_4 (.X (Math|Vector|BreakVector (Variables|Default|GetVelocity))) (Variables|Movement|GetLateralDragMultiplier)) (* _returnvalue_4 (.Y (Math|Vector|BreakVector (Variables|Default|GetVelocity)))) 0.0)) (Variables|Default|GetVelocity))) (Math|Float|Max(Float) (.y (+ (Math|Vector|NegateVector (Math|Vector|MakeVector (* _returnvalue_4 (.X (Math|Vector|BreakVector (Variables|Default|GetVelocity))) (Variables|Movement|GetLateralDragMultiplier)) (* _returnvalue_4 (.Y (Math|Vector|BreakVector (Variables|Default|GetVelocity)))) 0.0)) (Variables|Default|GetVelocity))) 0.0) 0.0) :!label _label)))
    (else
      (goto _label)))
  (Variables|Default|SetVelocity (Math|Vector|MakeVector (.x (Variables|Default|GetVelocity)) (Math|Float|SelectFloat 0.0 (Math|Float|Clamp(Float) (.y (Variables|Default|GetVelocity)) (Variables|Movement|GetMinSpeed) (Variables|Movement|GetMaxSpeed)) (Variables|Default|GetHasHitObstacle)) 0.0)))

(fn ConstructionScript)

(fn UpdateLocation
  (bind (_returnvalue_location _pad _as_bp_oar) (Utilities|GetBpOarPadRelativeLoc))
  (bind _paddledetectionthreshhold (Variables|Default|GetPaddleDetectionThreshHold))
  (Utilities|IsValid _as_bp_oar
    (:Is%20Valid
      (Variables|Default|SetForwardAcceleration (* (.x (Math|Vector|RotateVector (Math|Vector|NegateVector (- _returnvalue_location (Variables|Default|GetPreviousOarPos))) (Math|Rotator|MakeRotator 0.0 0.0 -9e+01))) (Math|Float|SelectFloat (Variables|Movement|GetMoveForce) 0.0 (or (> (.x (Math|Vector|RotateVector (Math|Vector|NegateVector (- _returnvalue_location (Variables|Default|GetPreviousOarPos))) (Math|Rotator|MakeRotator 0.0 0.0 -9e+01))) _paddledetectionthreshhold) (< (.x (Math|Vector|RotateVector (Math|Vector|NegateVector (- _returnvalue_location (Variables|Default|GetPreviousOarPos))) (Math|Rotator|MakeRotator 0.0 0.0 -9e+01))) (* _paddledetectionthreshhold -1.0))))))
      (Variables|Default|SetPreviousOarPos _returnvalue_location)
      (Variables|Default|SetIsPadInWater true))))

(fn UnlockPaddle
  (Variables|Default|SetIsPaddleLocked false)
  (Variables|Default|SetAs%20BP%20Oar 0)
  (Variables|Default|SetOarPaddle 0)
  (Utilities|Time|ClearandInvalidateTimerbyHandle (Variables|Default|GetUpdateRotationHandle))
  (Variables|Default|SetUpdateRotationHandle "")
  (Variables|Default|SetIsPadInWater false)
  (Variables|Default|SetForwardAcceleration 0.0)
  (Variables|Default|SetSidePaddled "Pad")
  (Development|PrintString "RELEASED" true true "(R=1.000000,G=0.081488,B=0.000000,A=1.000000)"))

(fn UpdateForwardPaddling
  (bind _forwardacceleration (Variables|Default|GetForwardAcceleration))
  (Variables|Default|SetVelocity (+ (Variables|Default|GetVelocity) (Math|Vector|MakeVector (* _forwardacceleration (Utilities|GetLateralMultiplier)) _forwardacceleration 0.0)))
  (return))

(fn UpdateBackwardPaddling
  (params (dt :type Float%20%28double-precision%29))
  (Variables|Default|SetVelocity (+ (Variables|Default|GetVelocity) (Math|Vector|MakeVector (* (Variables|Default|GetForwardAcceleration) (Utilities|GetLateralMultiplier) 0.8) (* (* dt (* (Variables|Movement|GetDragForce) (Variables|Movement|GetPaddleBreakingForceMultiplier))) (.y (Variables|Default|GetVelocity)) -1.0) 0.0)))
  (return))