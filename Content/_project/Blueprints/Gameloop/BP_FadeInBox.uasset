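; BP_FadeInBox is a mesh-based fade effect that, judging by its name, fades the view in when play begins.
; On BeginPlay it creates a dynamic instance of M_NormalFlip on its static mesh and sets opacity to 1.
; It then plays FadeOutTimeline in reverse from the end, feeding each update into the material's Opacity parameter through SetOpacity.
; The construction script also applies the Opacity variable, but only when a material instance already exists.
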(event EventBeginPlay
  (bind _returnvalue (Rendering|Material|CreateDynamicMaterialInstance (Variables|Default|GetStaticMesh) 0 "/Game/_project/Art/NormalFlip/M_NormalFlip.M_NormalFlip" "None" :!class /Script/Engine.PrimitiveComponent))
  (Variables|Default|SetMaterialInstance _returnvalue)
  (CallFunction|SetOpacity 1.0)
  (bind _newtrack_0 (Timeline|FadeOutTimeline ReverseFromEnd)
    (:Update
      (CallFunction|SetOpacity _newtrack_0))))

(fn ConstructionScript
  (CallFunction|SetOpacity (Variables|Default|GetOpacity)))

(fn SetOpacity
  (params (Value :type Float%20%28double-precision%29))
  (bind _materialinstance (Variables|Default|GetMaterialInstance)
    (:then
      (Rendering|Material|SetScalarParameterValue _materialinstance "Opacity" Value :!class /Script/Engine.MaterialInstanceDynamic))
    (:else)))