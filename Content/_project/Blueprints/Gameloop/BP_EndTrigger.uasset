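; BP_EndTrigger ends the level when a spline reports its end reached, then returns the player to the menu in VR.
; On BeginPlay it binds to the OnReachEnd event of every BP_Spline in the level, which plays the EndLevelSequencer sequence.
; When the sequence finishes, it shows a VR loading screen offset by headset height, waits briefly, and opens LD_Menu.
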(event Custom|CE_EndLevel
  (bind _endlevelsequencer (Variables|Default|GetEndLevelSequencer))
  (bind _sequenceplayer (Variables|/Script/LevelSequence.LevelSequenceActor|GetSequencePlayer _endlevelsequencer))
  (Sequencer|Player|Play _sequenceplayer :!class /Script/MovieScene.MovieSceneSequencePlayer)
  (EventDispatchers|BindEventtoOnFinished _sequenceplayer (delegate Custom|CE_TransitionMenu)))

(event Custom|CE_TransitionMenu
  (Class|XRLoadingScreenFunctionLibrary|SetLoadingScreen "/NiagaraFluids/Textures/VolumeTextures/VelocityRenderTarget.VelocityRenderTarget" "(X=4.000000,Y=4.000000)" (Math|Vector|MakeVector 1e+01 0.0 (/ (.Z (Math|Vector|BreakVector (.DevicePosition (Class|HeadMountedDisplayFunctionLibrary|GetOrientationandPosition)))) 1e+02)) false true) ; Offset values are in Meters
  (Utilities|FlowControl|Delay 3.0)
  (Game|OpenLevel(byObjectReference) "/Game/_project/Levels/LD_Menu.LD_Menu"))

(event EventBeginPlay
  (bind _outactors (Actor|GetAllActorsOfClass "/Game/_project/Blueprints/BP_Spline.BP_Spline_C"))
  (bind _array_element (Utilities|Array|ForEachLoopwithBreak _outactors)
    (:LoopBody
      (bind _asbp_spline (Utilities|Casting|CastToBP_Spline _array_element))
      (EventDispatchers|BindEventtoOnReachEnd _asbp_spline (delegate Custom|CE_EndLevel)))))

(fn ConstructionScript)