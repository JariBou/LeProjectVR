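; BP_WaterBody is a water body in the Buoyancy set that defines a directional current and animates its surface to match.
; On BeginPlay, it stores WaterFlow as the Arrow component's forward vector scaled by WaterPower.
; It then drives a dynamic material's Speed from WaterPower, with a slow fallback for non-positive power, and sets Direction opposite the arrow.
; The audio playback nodes are disconnected and never run.
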(event EventBeginPlay
  (bind _arrow (Variables|Default|GetArrow))
  (bind _waterpower (Variables|Default|GetWaterPower))
  (bind _returnvalue (Math|Vector|GetForwardVector _arrow))
  (Variables|Default|SetWaterFlow (* _returnvalue _waterpower))
  (bind _returnvalue_2 (Rendering|Material|CreateDynamicMaterialInstance (Variables|Default|GetTexture) 0 0 "None" :!class /Script/Engine.PrimitiveComponent))
  (if (> _waterpower 0.0)
    (Rendering|Material|SetScalarParameterValue _returnvalue_2 "Speed" (/ _waterpower 8e+02) :!class /Script/Engine.MaterialInstanceDynamic)
    (else
      (Rendering|Material|SetScalarParameterValue _returnvalue_2 "Speed" 0.025 :!class /Script/Engine.MaterialInstanceDynamic)))
  (Rendering|Material|SetVectorParameterValue _returnvalue_2 "Direction" (Math|Conversions|ToLinearColor(Vector) (Math|Vector|NegateVector _returnvalue)) :!class /Script/Engine.MaterialInstanceDynamic))

(fn ConstructionScript)