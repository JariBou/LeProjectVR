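; Actor component that floats its owner's "Prop"-tagged mesh in BP_WaterBody volumes, using "Buoyancy"-tagged meshes as sample points.
; Overlapping water spawns a mass-scaled emitter, sums flow from current bodies and raises the surface height.
; Each tick applies depth-scaled Archimedes lift, linear drag and angular drag per point, plus water flow.
; End overlap only removes the body from the list; in-water state, flow and height remain.
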(event Custom|Prop%20Begin%20Overlap
  (params (OverlappedComponent :type Primitive%20Component%20Object%20Reference) (OtherActor :type Actor%20Object%20Reference) (OtherComp :type Primitive%20Component%20Object%20Reference) (OtherBodyIndex :type Integer) (bFromSweep :type Boolean) (SweepResult :type Hit%20Result%20Structure%20%28by%20ref%29))
  (bind _cube (Variables|Default|GetCube))
  (bind _returnvalue (Transformation|GetWorldLocation _cube))
  (bind _returnvalue_2 (Physics|GetMass _cube))
  (bind _returnvalue_3 (/ _returnvalue_2 1e+02))
  (bind _asbp_water_body (Utilities|Casting|CastToBP_WaterBody OtherActor))
  (Utilities|Array|Add (Variables|Default|GetWaterBodyList) _asbp_water_body)
  (if (> _returnvalue_3 3.0)
    (Effects|SpawnEmitteratLocation 0 _returnvalue "0, 0, 0" "3.000000,3.000000,3.000000")
    (else
      (Effects|SpawnEmitteratLocation 0 _returnvalue "0, 0, 0" (Math|Conversions|ToVector(Float) _returnvalue_3))))
  (Variables|Default|SetWaterFlowForce "0, 0, 0")
  (for _array_element (Variables|Default|GetWaterBodyList)
    (Variables|Default|SetWaterFlowForce (+ (Variables|Default|GetWaterFlowForce) (Variables|/Game/_project/Blueprints/Buoyancy/BP_WaterBody.BP_WaterBody_C|GetWaterFlow _array_element)))
    (if (> (+ (.z (Transformation|GetWorldLocation (Variables|/Script/Engine.Actor|GetRootComponent _array_element))) (Variables|/Game/_project/Blueprints/Buoyancy/BP_WaterBody.BP_WaterBody_C|GetBoxZOffset _array_element)) (Variables|Default|GetWaterZTop))
      (Variables|Default|SetWaterZTop (+ (.z (Transformation|GetWorldLocation (Variables|/Script/Engine.Actor|GetRootComponent _array_element))) (Variables|/Game/_project/Blueprints/Buoyancy/BP_WaterBody.BP_WaterBody_C|GetBoxZOffset _array_element)))))
  (Variables|Default|SetInWater true))

(event Custom|Prop%20End%20Overlap
  (params (OverlappedComponent :type Primitive%20Component%20Object%20Reference) (OtherActor :type Actor%20Object%20Reference) (OtherComp :type Primitive%20Component%20Object%20Reference) (OtherBodyIndex :type Integer))
  (bind _asbp_water_body (Utilities|Casting|CastToBP_WaterBody OtherActor))
  (Utilities|Array|RemoveItem (Variables|Default|GetWaterBodyList) _asbp_water_body))

(event EventTick
  (params (DeltaSeconds :type Float%20%28single-precision%29))
  (bind _returnvalue (Utilities|Time|GetWorldDeltaSeconds))
  (bind _cube (Variables|Default|GetCube))
  (if (and (Variables|Default|GetInWater) (Variables|Default|GetBuoyancy))
    ;[1 0.8122 0.4064] Init Variables & Loop
    (for _array_element (Variables|Default|GetBuoList)
      ;[0.3017 0.4763 1] Archimedes' principle
      (Class|PrimitiveComponent|AddForceatLocation _cube (Math|Vector|MakeVector 0.0 0.0 (/ (* (* (Variables|Default|GetBuoAppliedForce) (Math|Float|Clamp(Float) (Math|Float|SafeDivide (- (Variables|Default|GetWaterZTop) (.z (+ (Transformation|GetWorldLocation _array_element) ""))) (Variables|Default|GetBuoDepth)) 0.0 1e+03) 0.1) (Math|Float|Absolute(Float) (Variables|Default|GetGravityZ))) (Variables|Default|GetBuoAmount))) (Transformation|GetWorldLocation _array_element) "None")
      ;[0.3992 0.3637 1] Fluid Drag Force
      (Class|PrimitiveComponent|AddForceatLocation _cube (Math|Vector|MakeVector (/ (.x (* _returnvalue (* (Variables|Default|GetBuoAppliedForce) (Math|Float|Clamp(Float) (Math|Float|SafeDivide (- (Variables|Default|GetWaterZTop) (.z (+ (Transformation|GetWorldLocation _array_element) ""))) (Variables|Default|GetBuoDepth)) 0.0 1e+03) 0.1) (Variables|Default|GetBuoDragForce) (Math|Vector|NegateVector (Transformation|GetComponentVelocity _cube)))) (Variables|Default|GetBuoAmount)) (/ (.y (* _returnvalue (* (Variables|Default|GetBuoAppliedForce) (Math|Float|Clamp(Float) (Math|Float|SafeDivide (- (Variables|Default|GetWaterZTop) (.z (+ (Transformation|GetWorldLocation _array_element) ""))) (Variables|Default|GetBuoDepth)) 0.0 1e+03) 0.1) (Variables|Default|GetBuoDragForce) (Math|Vector|NegateVector (Transformation|GetComponentVelocity _cube)))) (Variables|Default|GetBuoAmount)) (/ (.z (* _returnvalue (* (Variables|Default|GetBuoAppliedForce) (Math|Float|Clamp(Float) (Math|Float|SafeDivide (- (Variables|Default|GetWaterZTop) (.z (+ (Transformation|GetWorldLocation _array_element) ""))) (Variables|Default|GetBuoDepth)) 0.0 1e+03) 0.1) (Variables|Default|GetBuoDragForce) (Math|Vector|NegateVector (Transformation|GetComponentVelocity _cube)))) (Variables|Default|GetBuoAmount))) (Transformation|GetWorldLocation _array_element) "None")
      ;[0.4325 1 0.8735] Angular Drag Force
      (Class|PrimitiveComponent|AddTorqueinRadians _cube (Math|Vector|MakeVector (/ (.x (* _returnvalue (* (Variables|Default|GetBuoAppliedForce) (Math|Float|Clamp(Float) (Math|Float|SafeDivide (- (Variables|Default|GetWaterZTop) (.z (+ (Transformation|GetWorldLocation _array_element) ""))) (Variables|Default|GetBuoDepth)) 0.0 1e+03) 0.1) (Variables|Default|GetBuoAngularDragForce) (Math|Vector|NegateVector (Class|PrimitiveComponent|GetPhysicsAngularVelocityinRadians _cube "None")))) (Variables|Default|GetBuoAmount)) (/ (.y (* _returnvalue (* (Variables|Default|GetBuoAppliedForce) (Math|Float|Clamp(Float) (Math|Float|SafeDivide (- (Variables|Default|GetWaterZTop) (.z (+ (Transformation|GetWorldLocation _array_element) ""))) (Variables|Default|GetBuoDepth)) 0.0 1e+03) 0.1) (Variables|Default|GetBuoAngularDragForce) (Math|Vector|NegateVector (Class|PrimitiveComponent|GetPhysicsAngularVelocityinRadians _cube "None")))) (Variables|Default|GetBuoAmount)) (/ (.z (* _returnvalue (* (Variables|Default|GetBuoAppliedForce) (Math|Float|Clamp(Float) (Math|Float|SafeDivide (- (Variables|Default|GetWaterZTop) (.z (+ (Transformation|GetWorldLocation _array_element) ""))) (Variables|Default|GetBuoDepth)) 0.0 1e+03) 0.1) (Variables|Default|GetBuoAngularDragForce) (Math|Vector|NegateVector (Class|PrimitiveComponent|GetPhysicsAngularVelocityinRadians _cube "None")))) (Variables|Default|GetBuoAmount))) "None" true))
    (Physics|AddForce _cube (Variables|Default|GetWaterFlowForce) "None" true :!label _label)
    (elif (Variables|Default|GetInWater)
      (goto _label))))

(event EventBeginPlay
  (bind _returnvalue (Components|GetOwner))
  (bind _returnvalue_2 (Actor|GetComponentsbyTag _returnvalue "/Script/Engine.StaticMeshComponent" "Prop"))
  (bind _output (Utilities|Array|Get(acopy) _returnvalue_2))
  ;[1 0.1269 0.1448] Begin Initialization
  (Variables|Default|SetGravityZ -9.8e+02)
  (Variables|Default|SetWaterFlowForce "0, 0, 0")
  (bind _output_get (Variables|Default|SetBuoList (Actor|GetComponentsbyTag _returnvalue "/Script/Engine.StaticMeshComponent" "Buoyancy")))
  (bind _output_get_2 (Variables|Default|SetBuoAmount (Utilities|Array|Length _output_get)))
  (if (<= _output_get_2 0)
    (Variables|Default|SetBuoyancy false))
  (Utilities|IsValid _output
    (:Is%20Valid
      (Collision|BindEventtoOnComponentBeginOverlap _output (delegate Custom|Prop%20Begin%20Overlap))
      (Collision|BindEventtoOnComponentEndOverlap _output (delegate Custom|Prop%20End%20Overlap))
      (Variables|Default|SetCube _output))
    (:Is%20Not%20Valid
      (Development|PrintString "Buoyancy : No Prop recognized"))))