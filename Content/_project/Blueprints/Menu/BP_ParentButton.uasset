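; Base menu button that the player activates by holding an oar (BP_Oar) inside its box, with a radial loading indicator showing progress.
; Oar overlap plays a timeline that drives the WBP_RadialLoading widget, and leaving the box reverses it.
; The timeline's Finished output calls CE_OnDone, an empty event here that appears intended for child buttons to override.
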(event OnComponentBeginOverlap(Box)
  (params (OverlappedComponent :type Primitive%20Component%20Object%20Reference) (OtherActor :type Actor%20Object%20Reference) (OtherComp :type Primitive%20Component%20Object%20Reference) (OtherBodyIndex :type Integer) (bFromSweep :type Boolean) (SweepResult :type Hit%20Result%20Structure%20%28by%20ref%29))
  (Utilities|Casting|CastToBP_Oar OtherActor)
  (bind _newtrack_0 (Timeline|LoadingTimeline Play)
    (:Update
      (bind _radialloading (Variables|Default|GetRadialLoading)
        (:then
          (Default|UpdateLoading _radialloading _newtrack_0))
        (:else)))
    (:Finished
      (CallFunction|CEonDone))))

(event OnComponentEndOverlap(Box)
  (params (OverlappedComponent :type Primitive%20Component%20Object%20Reference) (OtherActor :type Actor%20Object%20Reference) (OtherComp :type Primitive%20Component%20Object%20Reference) (OtherBodyIndex :type Integer))
  (Utilities|Casting|CastToBP_Oar OtherActor)
  (bind _newtrack_0 (Timeline|LoadingTimeline Reverse)
    (:Update
      (bind _radialloading (Variables|Default|GetRadialLoading)
        (:then
          (Default|UpdateLoading _radialloading _newtrack_0))
        (:else)))
    (:Finished
      (CallFunction|CEonDone))))

(event Custom|CE_OnDone)

(event EventBeginPlay
  (bind _aswbp_radial_loading (Utilities|Casting|CastToWBP_RadialLoading (UserInterface|GetWidget (Variables|Default|GetLoadingWidget))))
  (bind _output_get (Variables|Default|SetRadialLoading _aswbp_radial_loading))
  (Default|UpdateLoading _output_get 0.0))

(fn ConstructionScript)