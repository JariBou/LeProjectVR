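; BP_MonolithEnvironment is a monolith environment prop whose emissive glow fades between an off and an on intensity.
; BeginPlay creates a dynamic material instance on the static mesh and sets it to the off intensity.
; EndFX plays a timeline that lerps Emissive_Intensity from off toward on along a curve, and CallFX reverses that timeline to fade it back.
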(event EventEndFX
  (bind _courbe (Timeline|AGOUGOUGAGA Play)
    (:Update
      _)
    (:Finished
      _))
  (Rendering|Material|SetScalarParameterValue (Variables|Default|GetDynamic) "Emissive_Intensity" (Math|Float|Lerp (Variables|Default|GetOffEmissivePower) (Variables|Default|GetOnEmissivePower) _courbe) :!class /Script/Engine.MaterialInstanceDynamic))

(event EventCallFX
  (bind _courbe (Timeline|AGOUGOUGAGA Reverse)
    (:Update
      _)
    (:Finished
      _))
  (Rendering|Material|SetScalarParameterValue (Variables|Default|GetDynamic) "Emissive_Intensity" (Math|Float|Lerp (Variables|Default|GetOffEmissivePower) (Variables|Default|GetOnEmissivePower) _courbe) :!class /Script/Engine.MaterialInstanceDynamic))

(event EventBeginPlay
  (bind _returnvalue (Rendering|Material|CreateDynamicMaterialInstance (Variables|Default|GetStaticMesh) 0 "/Game/Art/02_Material/STRU/MI_STRU_Monolith_Environment_01_Inst.MI_STRU_Monolith_Environment_01_Inst" "None" :!class /Script/Engine.PrimitiveComponent))
  (bind _output_get (Variables|Default|SetDynamic _returnvalue))
  (Rendering|Material|SetScalarParameterValue _output_get "Emissive_Intensity" (Variables|Default|GetOffEmissivePower) :!class /Script/Engine.MaterialInstanceDynamic))

(fn ConstructionScript)