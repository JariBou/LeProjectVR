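; Spline follower Blueprint that moves a Follower actor along a Spline to track a Followed actor.
; Each Tick it finds the distance along the spline at the Followed actor's location and places Follower at that spline point.
; FollowX, FollowY and FollowZ choose per axis whether to take the spline position or keep the current one.
; An optional LookAt flag rotates Follower to face the Followed actor.
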(event EventBeginPlay)

(event Collision|EventActorBeginOverlap
  (params (OtherActor :type Actor%20Object%20Reference)))

(event EventTick
  (params (DeltaSeconds :type Float%20%28single-precision%29))
  (bind _spline (Variables|Default|GetSpline))
  (bind _spline_2 (Variables|Default|GetSpline))
  (bind _follower (Variables|Default|GetFollower))
  (bind _followed (Variables|Default|GetFollowed))
  (bind _returnvalue (Transformation|GetActorLocation _follower))
  (bind _returnvalue_2 (Transformation|GetActorLocation _followed))
  (bind _returnvalue_3 (Class|SplineComponent|GetDistanceAlongSplineatLocation _spline _returnvalue_2 "World"))
  (bind _returnvalue_4 (Spline|GetLocationatDistanceAlongSpline _spline_2 _returnvalue_3 "World"))
  (Transformation|SetActorLocation (Variables|Default|GetFollower) (Math|Vector|MakeVector (Math|Float|SelectFloat (.x _returnvalue_4) (.x _returnvalue) (Variables|Default|GetFollowX)) (Math|Float|SelectFloat (.y _returnvalue_4) (.y _returnvalue) (Variables|Default|GetFollowY)) (Math|Float|SelectFloat (.z _returnvalue_4) (.z _returnvalue) (Variables|Default|GetFollowZ))) false false)
  (if (Variables|Default|GetLookAt)
    (Transformation|SetActorRotation (Variables|Default|GetFollower) (Math|Rotator|FindLookatRotation (Transformation|GetActorLocation (Variables|Default|GetFollower)) (Transformation|GetActorLocation (Variables|Default|GetFollowed))))))

(fn ConstructionScript)