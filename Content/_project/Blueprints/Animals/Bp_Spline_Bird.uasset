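; Spline-following bird actor that moves a Crow component along its Spline at a set speed.
; While Playing, Tick advances the distance and applies the local spline transform with sweep, offsetting yaw by -90 degrees and preserving scale.
; With Loop on, the distance resets to zero past the spline's end.
; Two generically named custom events start and stop playback.
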(event Custom|CustomEvent
  (Variables|Default|SetPlaying true))

(event Custom|CustomEvent_1
  (Variables|Default|SetPlaying false)
  (if (Variables|Default|GetLoop?)
    _))

(event EventTick
  (params (DeltaSeconds :type Float%20%28single-precision%29))
  (if (Variables|Default|GetPlaying)
    (Variables|Default|SetDistance%20Along%20Spline (+ (* DeltaSeconds (Variables|Default|GetSplineSpeed)) (Variables|Default|GetDistance%20Along%20Spline)))
    (Transformation|SetRelativeTransform (Variables|Default|GetCrow) (Math|Transform|MakeTransform (Math|Vector|MakeVector (.x (.location (Spline|GetTransformatDistanceAlongSpline (Variables|Default|GetSpline) (Variables|Default|GetDistance%20Along%20Spline) "Local" false))) (.y (.location (Spline|GetTransformatDistanceAlongSpline (Variables|Default|GetSpline) (Variables|Default|GetDistance%20Along%20Spline) "Local" false))) (.z (.location (Spline|GetTransformatDistanceAlongSpline (Variables|Default|GetSpline) (Variables|Default|GetDistance%20Along%20Spline) "Local" false)))) (Math|Rotator|MakeRotator (.roll (.rotation (Spline|GetTransformatDistanceAlongSpline (Variables|Default|GetSpline) (Variables|Default|GetDistance%20Along%20Spline) "Local" false))) (.pitch (.rotation (Spline|GetTransformatDistanceAlongSpline (Variables|Default|GetSpline) (Variables|Default|GetDistance%20Along%20Spline) "Local" false))) (+ (.yaw (.rotation (Spline|GetTransformatDistanceAlongSpline (Variables|Default|GetSpline) (Variables|Default|GetDistance%20Along%20Spline) "Local" false))) -9e+01)) (Variables|/Script/Engine.SceneComponent|GetRelativeScale3D (Variables|Default|GetCrow))) true false)
    (if (Variables|Default|GetLoop?)
      (if (> (Variables|Default|GetDistance%20Along%20Spline) (Spline|GetSplineLength (Variables|Default|GetSpline)))
        (Variables|Default|SetDistance%20Along%20Spline 0.0)))))

(fn ConstructionScript)