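; Crocodile actor that moves its Crocodil component along a spline and sinks it when its collide event fires.
; CallFX and EndFX toggle playback; while playing, Tick advances along the spline at SplineSpeed, applying position and yaw-corrected rotation, restarting at the end if Loop is set.
; OnCollide works once: it disables the Box collision and plays a timeline that blends a downward height offset to TargetHeightDiff.
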(event EventTick
  (params (DeltaSeconds :type Float%20%28single-precision%29))
  (if (Variables|Default|GetPlaying)
    (Variables|Default|SetDistance%20Along%20Spline (+ (* DeltaSeconds (Variables|Default|GetSplineSpeed)) (Variables|Default|GetDistance%20Along%20Spline)))
    (Transformation|SetRelativeTransform (Variables|Default|GetCrocodil) (Math|Transform|MakeTransform (Math|Vector|MakeVector (.x (.location (Spline|GetTransformatDistanceAlongSpline (Variables|Default|GetSpline) (Variables|Default|GetDistance%20Along%20Spline) "Local" false))) (.y (.location (Spline|GetTransformatDistanceAlongSpline (Variables|Default|GetSpline) (Variables|Default|GetDistance%20Along%20Spline) "Local" false))) (- (.z (.location (Spline|GetTransformatDistanceAlongSpline (Variables|Default|GetSpline) (Variables|Default|GetDistance%20Along%20Spline) "Local" false))) (Variables|Default|GetCurrEightOffset))) (Math|Rotator|MakeRotator (.roll (.rotation (Spline|GetTransformatDistanceAlongSpline (Variables|Default|GetSpline) (Variables|Default|GetDistance%20Along%20Spline) "Local" false))) (.pitch (.rotation (Spline|GetTransformatDistanceAlongSpline (Variables|Default|GetSpline) (Variables|Default|GetDistance%20Along%20Spline) "Local" false))) (+ (.yaw (.rotation (Spline|GetTransformatDistanceAlongSpline (Variables|Default|GetSpline) (Variables|Default|GetDistance%20Along%20Spline) "Local" false))) -9e+01)) (Variables|/Script/Engine.SceneComponent|GetRelativeScale3D (Variables|Default|GetCrocodil))) true false)
    (if (Variables|Default|GetLoop?)
      (if (> (Variables|Default|GetDistance%20Along%20Spline) (Spline|GetSplineLength (Variables|Default|GetSpline)))
        (Variables|Default|SetDistance%20Along%20Spline 0.0)))))

(event EventOnCollide
  (if (Variables|Default|GetEnabled)
    (Collision|SetCollisionEnabled (Variables|Default|GetBox) "NoCollision")
    (Variables|Default|SetEnabled false)
    (bind _t (Timeline|BigBoomShakalakaCrocodileVersion Play)
      (:Update
        (Variables|Default|SetCurrEightOffset (Math|Float|Lerp 0.0 (Variables|Default|GetTargetHeightDiff) _t))))))

(event EventCallFX
  (Variables|Default|SetPlaying true))

(event EventEndFX
  (Variables|Default|SetPlaying false)
  (if (Variables|Default|GetLoop?)
    _))

(fn ConstructionScript)