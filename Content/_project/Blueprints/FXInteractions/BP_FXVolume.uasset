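; BP_FXVolume is an FX trigger volume that plays Niagara and audio, started either by overlap or, with EyeDetection, by CallFX/EndFX events.
; PlayFX and StopFX also forward those events to a SpecialInteraction implementing BPI_FXInteraction.
; Tick ramps audio in; on exit, it decrements only while above the transition time, then stops, so fade-out is negligible.
; CanPlay gates starts, but its one-shot check appears unconnected.
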(event EventCallFX
  ;[0.02808 0.15 0.01809 0.5] Enter Volume
  (if (and (Utilities|CanPlay) (Variables|Default|GetEyeDetection))
    (CallFunction|PlayFX)
    (Development|PrintString "Start FX by Eye" true true "(R=0.000000,G=0.573958,B=0.073829,A=1.000000)" 5.0)
    (else
      (Development|PrintString "Failed: Start FX by Eye" true true "(R=0.573958,G=0.246663,B=0.000000,A=1.000000)" 5.0))))

(event Collision|EventActorBeginOverlap
  (params (OtherActor :type Actor%20Object%20Reference))
  ;[0.02808 0.15 0.01809 0.5] Enter Volume
  (if (and (Utilities|CanPlay) (not (Variables|Default|GetEyeDetection)))
    (CallFunction|PlayFX)
    (Development|PrintString "Start FX by Overlap" true true "(R=0.000000,G=0.573958,B=0.073829,A=1.000000)" 5.0)
    (else
      (Development|PrintString "Failed: Start FX by Overlap" true true "(R=0.000000,G=0.573958,B=0.385901,A=1.000000)" 5.0))))

(event Collision|EventActorEndOverlap
  (params (OtherActor :type Actor%20Object%20Reference))
  ;[0.15 0.1243 0 0.5] Exit Volume
  (if (and (Variables|Default|GetCanDeactivate) (not (Variables|Default|GetEyeDetection)))
    (CallFunction|StopFX)
    (Variables|Default|SetPlaying false)
    (Development|PrintString "End FX by Overlap" true true "(R=0.573958,G=0.500882,B=0.000000,A=1.000000)" 5.0)
    (else
      (Development|PrintString "Failed: End FX by Overlap" true true "(R=0.573958,G=0.246663,B=0.000000,A=1.000000)" 5.0))))

(event EventBeginPlay
  (Variables|Default|SetVolume (Variables|/Script/Engine.AudioComponent|GetVolumeMultiplier (Variables|Default|GetAudio))))

(event EventTick
  (params (DeltaSeconds :type Float%20%28single-precision%29))
  (if (Variables|Default|GetPlaying)
    ;[0.2052 1 0.206 0.5] EnterVolumeTransition
    (if (< (Variables|Default|GetCurrentTime) (Variables|Default|GetVolumeTransitionTime))
      (bind _output_get (Variables|Default|SetCurrentTime (+ DeltaSeconds (Variables|Default|GetCurrentTime))))
      (Audio|Components|Audio|SetVolumeMultiplier (Variables|Default|GetAudio) (* (/ _output_get (Variables|Default|GetVolumeTransitionTime)) (Variables|Default|GetVolume)) :!class /Script/Engine.AudioComponent)
      (else
        (Audio|Components|Audio|SetVolumeMultiplier (Variables|Default|GetAudio) (Variables|Default|GetVolume) :!class /Script/Engine.AudioComponent)))
    (else
      ;[0.8198 0.7858 0.04353 0.5] ExitVolumeTransition
      (if (> (Variables|Default|GetCurrentTime) (Variables|Default|GetVolumeTransitionTime))
        (bind _output_get_2 (Variables|Default|SetCurrentTime (- (Variables|Default|GetCurrentTime) DeltaSeconds)))
        (Audio|Components|Audio|SetVolumeMultiplier (Variables|Default|GetAudio) (* (/ _output_get_2 (Variables|Default|GetVolumeTransitionTime)) (Variables|Default|GetVolume)) :!class /Script/Engine.AudioComponent)
        (else
          (Audio|Components|Audio|Stop (Variables|Default|GetAudio)))))))

(event EventEndFX
  ;[0.15 0.1243 0 0.5] Exit Volume
  (if (and (Variables|Default|GetCanDeactivate) (Variables|Default|GetEyeDetection))
    (CallFunction|StopFX)
    (Variables|Default|SetPlaying false)
    (Development|PrintString "End FX by Eye" true true "(R=0.573958,G=0.500882,B=0.000000,A=1.000000)" 5.0)
    (else
      (Development|PrintString "Failed: End FX by Eye" true true "(R=0.573958,G=0.246663,B=0.000000,A=1.000000)" 5.0))))

(fn ConstructionScript)

(fn PlayFX
  (bind _audio (Variables|Default|GetAudio))
  (Components|Activation|Activate (Variables|Default|GetNiagara) (Variables|Default|GetOneShot))
  (if (Audio|Components|Audio|IsPlaying _audio)
    _
    (else
      (Audio|Components|Audio|Play _audio 0.0)))
  (if (Utilities|DoesObjectImplementInterface (Variables|Default|GetSpecialInteraction) "/Game/_project/Blueprints/FXInteractions/BPI_FXInteraction.BPI_FXInteraction_C")
    (CallFunction|CallFX))
  (Variables|Default|SetPlayed true)
  (Variables|Default|SetPlaying true))

(fn StopFX
  (Components|Activation|Deactivate (Variables|Default|GetNiagara))
  (if (Utilities|DoesObjectImplementInterface (Variables|Default|GetSpecialInteraction) "/Game/_project/Blueprints/FXInteractions/BPI_FXInteraction.BPI_FXInteraction_C")
    (CallFunction|EndFX))
  (return))